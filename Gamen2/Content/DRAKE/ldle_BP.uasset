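; ldle_BP is an attacker Blueprint that damages the player through a right-arm collision component.
; AttackEvent stores the damage amount and toggles the arm's collision for the attack window, which starts disabled on BeginPlay.
; When the arm begins overlapping player character 0, it applies the stored damage.
; Damage received by the actor is only printed as a string.
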(event OnComponentBeginOverlap(RIghtArm)
  (params (OverlappedComponent :type Primitive%20Component%20Object%20Reference) (OtherActor :type Actor%20Object%20Reference) (OtherComp :type Primitive%20Component%20Object%20Reference) (OtherBodyIndex :type Integer) (bFromSweep :type Boolean) (SweepResult :type Hit%20Result%20Structure%20%28by%20ref%29))
  (if (== OtherActor (Game|GetPlayerCharacter 0))
    (Game|Damage|ApplyDamage (Game|GetPlayerCharacter 0) (Variables|Default|GetDamage) 0 0)))

(event EventBeginPlay
  (Collision|SetCollisionEnabled (Variables|Default|GetRIght%20Arm) "NoCollision"))

(event Game|Damage|EventAnyDamage
  (params (Damage :type Float%20%28single-precision%29) (DamageType :type Damage%20Type%20Object%20Reference) (InstigatedBy :type Controller%20Object%20Reference) (DamageCauser :type Actor%20Object%20Reference))
  (Development|PrintString (Utilities|String|ToString(Float) Damage) false false))

(event EventAttackEvent
  (params (Damage :type Float%20%28single-precision%29) (ls%20Begin? :type Boolean))
  (Variables|Default|SetDamage Damage)
  (if ls%20Begin?
    (Collision|SetCollisionEnabled (Variables|Default|GetRIght%20Arm) "QueryAndPhysics")
    (else
      (Collision|SetCollisionEnabled (Variables|Default|GetRIght%20Arm) "NoCollision"))))

(fn ConstructionScript)